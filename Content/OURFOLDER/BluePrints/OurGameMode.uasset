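; OurGameMode is a game mode Blueprint that restarts the game when the player character is destroyed.
; On BeginPlay it casts player character 0 to NewPlayer and binds an event to that actor's destruction.
; The event waits briefly, then reloads by opening Example_Map by name.
; Unconnected nodes for spawning BrainFlipBlue and respawning and possessing a new NewPlayer remain in the graph but never run.
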(event `self.ReceiveBeginPlay`
  (bind _asnewplayer_c (cast `/Game/OURFOLDER/BluePrints/Player/NewPlayer` (`GameplayStatics.GetPlayerCharacter` 0)))
  (add `self.OnDestroyed` _asnewplayer_c (delegate `OnDestroyEvent`)))

(event `OnDestroyEvent`
  (`KismetSystemLibrary.Delay` 0.2)
  (`GameplayStatics.OpenLevel` "Example_Map"))

(fn `UserConstructionScript`)