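; BrainFlipBlue2 is a flipbook-based enemy that, on an overlap with its head box, adds a small amount to the player's health and destroys itself.
; The overlap event takes player 0's controlled pawn, cast to NewPlayer, without checking which actor overlapped.
; Timeline movement between PA and PB, scale-based sprite flipping and a debug print remain in the graph but are disconnected, so they never run.
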(event `self.Box Head.OnComponentBeginOverlap`
  (params (OtherActor :type "Actor Object Reference") (OtherComp :type "PrimitiveComponent Object Reference") (OtherBodyIndex :type Integer) (bFromSweep :type Boolean) (SweepResult :type "EngineTypes.HitResult Structure (by ref)"))
  (bind _asnewplayer_c (cast `/Game/OURFOLDER/BluePrints/Player/NewPlayer` (`Controller.K2_GetPawn` (`GameplayStatics.GetPlayerController` 0))))
  (set `/Game/OURFOLDER/BluePrints/Player/NewPlayer.PlayerHealth` (+ (`/Game/OURFOLDER/BluePrints/Player/NewPlayer.PlayerHealth` _asnewplayer_c) 0.2) _asnewplayer_c)
  (`self.K2_DestroyActor`))

(event `self.ReceiveBeginPlay`)

(fn `UserConstructionScript`)