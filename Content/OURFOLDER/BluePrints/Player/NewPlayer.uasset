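; Player character for a side-scrolling platformer, with X-axis movement, a launch-based double jump and a mouse-aimed grapple hook.
; Q and E teleport the character along Y between background planes through DoOnce gates, some reset by R.
; While left mouse is held, Tick stores the cursor hit, updates a child CableActor's cable and interpolates the character toward it.
; Health, death and level-loading logic is left unconnected.
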(event `self.ReceiveBeginPlay`
  (`ActorComponent.SetIsReplicated` (`self.PaperSprite1`) true))

(event `self.ReceiveActorBeginOverlap`
  (params (OtherActor :type "Actor Object Reference")))

(event `InputAxis|MoveRight`
  (params (AxisValue :type "Float (single-precision)"))
  ;[1 1 1] Movement
  (`self.AddMovementInput` (1.0 0.0 0.0) AxisValue))

(event `InputAxis|MoveArrows`
  (params (AxisValue :type "Float (single-precision)"))
  ;[1 1 1] Movement
  (`self.AddMovementInput` (1.0 0.0 0.0) AxisValue))

(event `Key|H`)

(event `Key|Q`
  ;[1 1 1] Moving into background
  (:`Pressed`
    (`/Engine/EditorBlueprintResources/StandardMacros.DoOnce` false :!label _label
      (:`Completed`
        (`self.K2_TeleportTo` :`self` (`GameplayStatics.GetPlayerCharacter` 0) :`DestLocation` (+ (`self.K2_GetActorLocation`) (0.0 -5000.0 0.0)))))))

(event `InputAction|Jump`
  ;[1 1 1] Double Jump
  (:`Pressed`
    (bind _counter (`/Engine/EditorBlueprintResources/StandardMacros.Do N` 2 :!label _label_2)
      (:`Exit`
        (switch `int` _counter
          (:`1`
            (`self.LaunchCharacter` (0.0 0.0 725.0) false true))
          (:`2`
            (`self.LaunchCharacter` (0.0 0.0 725.0) false true)))))))

(event `Key|Q`
  ;[1 1 1] Moving into background
)

(event `Key|E`
  ;[1 1 1] Moving into background
)

(event `Key|E`
  (:`Pressed`
    (`/Engine/EditorBlueprintResources/StandardMacros.DoOnce` false
      (:`Completed`
        (`self.K2_TeleportTo` :`self` (`GameplayStatics.GetPlayerCharacter` 0) :`DestLocation` (+ (`self.K2_GetActorLocation`) (0.0 -10000.0 0.0)))))))

(event `Key|Y`)

(event `Key|R`
  ;[1 1 1] Moving into background
  (:`Pressed`
    (goto _label :!via `Reset`)))

(event `self.OnLanded`
  (params (Hit :type "EngineTypes.HitResult Structure (by ref)"))
  ;[1 1 1] Double Jump
  (goto _label_2 :!via `Reset`))

(event `Key|E`)

(event `Key|Y`)

(event `self.Destroy Enemy Box.OnComponentBeginOverlap`
  (params (OtherActor :type "Actor Object Reference") (OtherComp :type "PrimitiveComponent Object Reference") (OtherBodyIndex :type Integer) (bFromSweep :type Boolean) (SweepResult :type "EngineTypes.HitResult Structure (by ref)")))

(event `Key|E`
  ;[1 1 1] Moving into background
)

(event `Key|H`)

(event `Key|Q`
  ;[1 1 1] Moving into background
)

(event `Key|E`
  (:`Pressed`
    (`/Engine/EditorBlueprintResources/StandardMacros.DoOnce` false :!via `Reset`
      (:`Completed`
        (`self.K2_TeleportTo` :`self` (`GameplayStatics.GetPlayerCharacter` 0) :`DestLocation` (+ (`self.K2_GetActorLocation`) (0.0 10000.0 0.0)))))))

(event `Key|Q`
  ;[1 1 1] Moving into background
  (:`Pressed`
    (goto _label_3 :!via `Reset`)))

(event `Key|R`
  ;[1 1 1] Moving into background
  (:`Pressed`
    (`/Engine/EditorBlueprintResources/StandardMacros.DoOnce` false :!label _label_3
      (:`Completed`
        (`self.K2_TeleportTo` :`self` (`GameplayStatics.GetPlayerCharacter` 0) :`DestLocation` (+ (`self.K2_GetActorLocation`) (0.0 5000.0 0.0)))))))

(event `Key|E`)

(event `ReceiveBeginPlay_Copy`
  ;[1 1 1] Cable Actor Initialised
  (bind _ascableactor (cast `CableActor` (`ChildActorComponent.ChildActor` (`self.Cable Actor`))))
  (bind _cablecomponent (`CableActor.CableComponent` _ascableactor))
  (`SceneComponent.SetVisibility` _cablecomponent false false)
  (set `CableComponent.CableWidth` 10.0 _cablecomponent)
  (set `CableComponent.EndLocation` (0.0 0.0 0.0) _cablecomponent)
  (set `CableComponent.CableLength` 0.0 _cablecomponent)
  (set `CableComponent.SolverIterations` 2 _cablecomponent)
  (set `self.Grapple Cmpt` _cablecomponent))

(event `self.ReceiveTick`
  (params (DeltaSeconds :type "Float (single-precision)"))
  (bind _returnvalue (`GameplayStatics.GetPlayerController` 0))
  (bind _returnvalue_2 (`GameplayStatics.GetPlayerController` 0))
  (bind _returnvalue_3 (`self.K2_GetActorLocation`))
  (bind _capsulecomponent (`self.CapsuleComponent`))
  (bind _grapple_cmpt (`self.Grapple Cmpt`))
  (bind _grapple_cmpt_2 (`self.Grapple Cmpt`))
  (bind _lasthook (`self.LastHook`))
  (bind _lasthook_2 (`self.LastHook`))
  (bind _grappledistance (`self.grappleDistance`))
  (bind _returnvalue_4 (`SceneComponent.K2_GetComponentLocation` _capsulecomponent))
  (bind (_hitresult _returnvalue_5) (`PlayerController.GetHitResultUnderCursorByChannel` _returnvalue_2 "TraceTypeQuery1" false))
  (bind _endlocation (`CableComponent.EndLocation` _grapple_cmpt))
  (bind _location (`GameplayStatics.BreakHitResult` _hitresult))
  (bind _returnvalue_6 (`KismetMathLibrary.LessLess_VectorRotator` (- _lasthook (`self.K2_GetActorLocation`)) (`self.K2_GetActorRotation`)))
  (bind _returnvalue_7 (+ (`PlayerController.DeprojectMousePositionToWorld` _returnvalue) (`KismetMathLibrary.GreaterGreater_VectorRotator` (0.0 0.0 0.0) (`SceneComponent.K2_GetComponentRotation` _capsulecomponent))))
  (bind _returnvalue_8 (`KismetMathLibrary.VSize` (- _returnvalue_6 _endlocation)))
  (set `self.Delta Time` DeltaSeconds)
  (`|ExecutionSequence`
    (:`then_0`
      ;[1 1 1] Grapple Hook
      (if (and (`PlayerController.IsInputKeyDown` _returnvalue_2 "LeftMouseButton") (== (`self.LastHook`) (0.0 0.0 0.0)))
        (if (and (< (`KismetMathLibrary.VSize` (- (`self.K2_GetActorLocation`) _location)) 100000.0) _returnvalue_5)
          ;[0.4915 1 0.3925] Update Hook
          (set `self.LastHook` _location)
          (set `CableComponent.EndLocation` (0.0 0.0 0.0) _grapple_cmpt_2)
          (set `CableComponent.CableLength` 0.0 _grapple_cmpt_2)
          (set `CableComponent.SolverIterations` 5 _grapple_cmpt_2)
          (`SceneComponent.SetVisibility` _grapple_cmpt_2 true false)
          (set `self.hooked` true)
          (else
            ;[1 0.1689 0.1498] Reset Hook
            (set `self.LastHook` (0.0 0.0 0.0) :!label _label_4)
            (set `CableComponent.EndLocation` (0.0 0.0 0.0) _grapple_cmpt_2)
            (set `CableComponent.SolverIterations` 5 _grapple_cmpt_2)
            (`SceneComponent.SetVisibility` _grapple_cmpt_2 false false)))))
    (:`then_1`
      ;[1 1 1] Updating end hook Location
      (if (and (`PlayerController.IsInputKeyDown` (`GameplayStatics.GetPlayerController` 0) "LeftMouseButton") (!= _lasthook (0.0 0.0 0.0)))
        (if (`self.hooked`)
          (set `CableComponent.EndLocation` _returnvalue_6 _grapple_cmpt)
          (else
            (set `CableComponent.EndLocation` (`KismetMathLibrary.VInterpTo` _endlocation _returnvalue_6 (`self.Delta Time`) 1.0) _grapple_cmpt)))
        (if (> _returnvalue_8 (* _grappledistance 0.99))
          (set `self.hooked` true)
          (elif (== _grappledistance 0.0)
            (set `self.grappleDistance` _returnvalue_8)
            (elif (< _grappledistance 1500.0)
              (set `CableComponent.SolverIterations` 1 (`self.Grapple Cmpt`)))))))
    (:`then_2`
      ;[1 1 1] Move Charcter to Hook Location
      (if (and (`PlayerController.IsInputKeyDown` (`GameplayStatics.GetPlayerController` 0) "LeftMouseButton") (!= _lasthook_2 (0.0 0.0 0.0)))
        (`self.K2_SetActorLocation` (`KismetMathLibrary.VInterpTo` _returnvalue_3 _lasthook_2 (`self.Delta Time`) 10.0) (< (`KismetMathLibrary.VSize` (- _lasthook_2 _returnvalue_3)) 1000.0))))
    (:`then_3`
      ;[1 1 1] Cast to object
      (if (`self.IsGrappling`) :!label _label_5
        (cast `Pawn` (`Controller.K2_GetPawn` _returnvalue))
        (`KismetSystemLibrary.DrawDebugLine` _returnvalue_4 _returnvalue_7 (struct :`R` 0.99 :`G` 0.203425 :`A` 1.0) 0.0 10.0)
        (`KismetSystemLibrary.LineTraceSingleForObjects` _returnvalue_4 _returnvalue_7 (`|MakeArray` "ObjectTypeQuery1" "ObjectTypeQuery2" "ObjectTypeQuery3" :!type "EngineTypes.EObjectTypeQuery Enum"))))))

(event `Key|LeftMouseButton`
  ;[1 0.1689 0.1498] Reset Hook
  (:`Released`
    (goto _label_4)))

(event `Key|LeftMouseButton`
  ;[1 1 1] Cast to object
  (:`Pressed`
    (set `self.IsGrappling` true)
    (goto _label_5))
  (:`Released`
    (set `self.IsGrappling` false)
    (goto _label_5)))

(fn `UserConstructionScript`)