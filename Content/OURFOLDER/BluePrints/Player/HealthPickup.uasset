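; HealthPickup is a pickup actor that restores the player's health when something overlaps its HealthMesh.
; The overlap event ignores the overlapping actor and casts player pawn 0 to NewPlayer, then edits PlayerHealth directly.
; At or below a health threshold it adds a large boost and destroys itself.
; Above the threshold it adds a smaller boost without clamping and stays in the level.
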(event `self.HealthMesh.OnComponentBeginOverlap`
  (params (OtherActor :type "Actor Object Reference") (OtherComp :type "PrimitiveComponent Object Reference") (OtherBodyIndex :type Integer) (bFromSweep :type Boolean) (SweepResult :type "EngineTypes.HitResult Structure (by ref)"))
  (bind _asnewplayer_c (cast `/Game/OURFOLDER/BluePrints/Player/NewPlayer` (`GameplayStatics.GetPlayerPawn` 0)))
  (bind _playerhealth (`/Game/OURFOLDER/BluePrints/Player/NewPlayer.PlayerHealth` _asnewplayer_c))
  (if (<= _playerhealth 0.8)
    (set `/Game/OURFOLDER/BluePrints/Player/NewPlayer.PlayerHealth` (+ _playerhealth 0.5) _asnewplayer_c)
    (`self.K2_DestroyActor`)
    (else
      (set `/Game/OURFOLDER/BluePrints/Player/NewPlayer.PlayerHealth` (+ (`/Game/OURFOLDER/BluePrints/Player/NewPlayer.PlayerHealth` _asnewplayer_c) 0.2) _asnewplayer_c))))

(fn `UserConstructionScript`)