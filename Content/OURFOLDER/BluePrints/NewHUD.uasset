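; NewHUD is a HUD Blueprint that draws a mouse-following crosshair and puts the player's health widget on screen.
; BeginPlay creates the NEWHealth widget for player 0 and adds it to the viewport.
; DrawHUD draws the crosshair texture centered on the mouse position every frame.
; EnemyHitFunc opens or closes a gate with no visible output, and disconnected text and texture draw nodes remain unused.
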(event `self.ReceiveDrawHUD`
  (params (SizeX :type Integer) (SizeY :type Integer))
  (bind (_locationx _locationy) (`PlayerController.GetMousePosition` (`GameplayStatics.GetPlayerController` 0)))
  (`self.DrawTexture` "/Game/OURFOLDER/Sprites/crosshairfix.crosshairfix" (- _locationx 10.0) (- _locationy 10.0) 20.0 20.0 0.0 0.0 1.0 1.0 (struct :`R` 1.0 :`G` 1.0 :`B` 1.0 :`A` 1.0) "BLEND_Translucent" 1.0))

(event `self.ReceiveBeginPlay`
  (bind _returnvalue (`WidgetBlueprintLibrary.Create` "/Game/OURFOLDER/BluePrints/Widgets/NEWHealth.NEWHealth_C" (`GameplayStatics.GetPlayerController` 0)))
  (`UserWidget.AddToViewport` _returnvalue))

(event `self.EnemyHitFunc`
  (params (EnemyHit :type Boolean))
  (if EnemyHit
    (`/Engine/EditorBlueprintResources/StandardMacros.Gate` true :!via `Open` :!label _label)
    (else
      (goto _label :!via `Close`))))

(event `InputAxisKey|MouseX`
  (params (AxisValue :type "Float (single-precision)")))

(event `InputAxisKey|MouseY`
  (params (AxisValue :type "Float (single-precision)")))

(fn `UserConstructionScript`)